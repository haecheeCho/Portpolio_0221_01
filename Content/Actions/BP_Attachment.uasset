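; BP_Attachment is an attachment actor whose shape components detect other characters for its action objects.
; On BeginPlay it disables collision on all shapes and binds their overlap events, with OnCollision and OffCollision toggling them.
; Overlaps ignore the owner and actors of the owner's class, then forward Characters to DoAction, DoAirAction and DoSpecialAction as begin or end notifications.
; Equip and unequip events are empty stubs.
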(event Custom|BeginOverlap
  (params (OverlappedComponent :type Primitive%20Component%20Object%20Reference) (OtherActor :type Actor%20Object%20Reference) (OtherComp :type Primitive%20Component%20Object%20Reference) (OtherBodyIndex :type Integer) (bFromSweep :type Boolean) (SweepResult :type Hit%20Result%20Structure%20%28by%20ref%29))
  (bind _returnvalue (Components|GetOwner))
  (if (and (!= OtherActor _returnvalue) (!= (Utilities|GetClass OtherActor) (Utilities|GetClass _returnvalue)))
    (bind _ascharacter (Utilities|Casting|CastToCharacter OtherActor))
    (Default|OnAttachmentBeginOverlap (Variables|Default|GetDoAction) _ascharacter)
    (Default|OnAttachmentBeginOverlap (Variables|Default|GetDoAirAction) _ascharacter)
    (Default|OnAttachmentBeginOverlap (Variables|Default|GetDoSpecialAction) _ascharacter)))

(event Custom|EndOverlap
  (params (OverlappedComponent :type Primitive%20Component%20Object%20Reference) (OtherActor :type Actor%20Object%20Reference) (OtherComp :type Primitive%20Component%20Object%20Reference) (OtherBodyIndex :type Integer))
  (bind _returnvalue (Components|GetOwner))
  (if (and (!= OtherActor _returnvalue) (!= (Utilities|GetClass OtherActor) (Utilities|GetClass _returnvalue)))
    (bind _ascharacter (Utilities|Casting|CastToCharacter OtherActor))
    (Default|OnAttachmentEndOverlap (Variables|Default|GetDoAction) _ascharacter)
    (Default|OnAttachmentEndOverlap (Variables|Default|GetDoAirAction) _ascharacter)
    (Default|OnAttachmentEndOverlap (Variables|Default|GetDoSpecialAction) _ascharacter)))

(event Custom|OffEquip)

(event Custom|OnUnequip)

(event Custom|OnEquip)

(event EventBeginPlay
  (Utilities|FlowControl|Sequence
    (:then_0
      (CallFunction|OffCollision))
    (:then_1
      (for _array_element (Actor|GetComponentsByClass "/Script/Engine.ShapeComponent")
        (Collision|BindEventtoOnComponentBeginOverlap _array_element (delegate Custom|BeginOverlap))))
    (:then_2
      (for _array_element_2 (Actor|GetComponentsByClass "/Script/Engine.ShapeComponent")
        (Collision|BindEventtoOnComponentEndOverlap _array_element_2 (delegate Custom|EndOverlap))))))

(fn ConstructionScript)

(fn OnCollision
  (for _array_element (Actor|GetComponentsByClass "/Script/Engine.ShapeComponent")
    (Collision|SetCollisionEnabled _array_element "QueryAndPhysics")))

(fn OffCollision
  (for _array_element (Actor|GetComponentsByClass "/Script/Engine.ShapeComponent")
    (Collision|SetCollisionEnabled _array_element "NoCollision")))