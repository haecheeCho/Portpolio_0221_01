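; Warp action that teleports the owning character to a location under the mouse cursor.
; While equipped, Tick traces WorldStatic objects under the cursor to place and orient a targeting decal from the ActionComponent's attachment.
; DoAction starts only from idle with a valid hit, and Begin attaches a warp particle to the mesh.
; End moves the character to Location, which Tick keeps updating while equipped, then restores idle and movement.
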(event EventTick
  (params (DeltaSeconds :type Float%20%28single-precision%29))
  (bind _returnvalue (CallFunction|GetDecal))
  (if (CallFunction|GetEquipped)
    (bind _returnvalue_2 (CallFunction|GetCursorLocationandRotation (Variables|Default|GetLocation) (Variables|Default|GetRotation)))
    (if _returnvalue_2
      (Utilities|IsValid _returnvalue
        (:Is%20Valid
          (Rendering|SetVisibility _returnvalue true false)
          (Transformation|SetWorldLocation (CallFunction|GetDecal) (Variables|Default|GetLocation) false false)
          (Transformation|SetWorldRotation (CallFunction|GetDecal) (Variables|Default|GetRotation) false false)))
      (else
        (Utilities|IsValid _returnvalue
          (:Is%20Valid
            (Rendering|SetVisibility _returnvalue false false)))))))

(fn ConstructionScript
  (|CallParentFunction))

(fn DoAction
  (bind _state (Variables|Default|GetState))
  (|CallParentFunction)
  (if (Default|IsIdleMode _state)
    (bind _returnvalue (CallFunction|GetCursorLocationandRotation (Variables|Default|GetLocation) (Variables|Default|GetRotation)))
    (if _returnvalue
      (Default|SetActionMode _state)
      (CallFunction|PlayAction))))

(fn BeginDoAction
  (|CallParentFunction)
  (Effects|SpawnEmitterAttached "/Game/Effects/P_Warp.P_Warp" (Variables|/Script/Engine.Character|GetMesh (Variables|Default|GetOwnerCharacter)) "None"))

(fn EndDoAction
  (|CallParentFunction)
  (Transformation|SetActorLocation (Variables|Default|GetOwnerCharacter) (Variables|Default|GetLocation) false false)
  (Default|SetIdleMode (Variables|Default|GetState))
  (Default|SetMove (Variables|Default|GetStatus)))

(fn GetDecal
  (bind _ownercharacter (Variables|Default|GetOwnerCharacter))
  (bind _returnvalue (Actor|GetComponentbyClass _ownercharacter "/Game/Components/ActionComponent.ActionComponent_C"))
  (bind _attachment (Default|GetAttachment _returnvalue))
  (bind _returnvalue_2 (Actor|GetComponentbyClass _attachment "/Script/Engine.DecalComponent"))
  (Utilities|IsValid _returnvalue
    (:Is%20Valid
      (Utilities|IsValid _returnvalue_2
        (:Is%20Valid
          (return _returnvalue_2))))))

(fn GetCursorLocationandRotation
  (params (OutLocation :type Vector%20%28by%20ref%29) (OutRotation :type Rotator%20%28by%20ref%29))
  (bind _returnvalue (Game|GetPlayerController 0))
  (bind _array (Utilities|Array|MakeArray "ObjectTypeQuery1"))
  (bind (_hitresult _returnvalue_2) (Class|PlayerController|GetHitResultUnderCursorforObjects _returnvalue _array false))
  (bind (_bblockinghit _binitialoverlap _time _distance _location _impactpoint _normal _impactnormal) (Collision|BreakHitResult _hitresult))
  (|SetBy-RefVar OutLocation _location)
  (|SetBy-RefVar OutRotation (Class|KismetMathLibrary|QuatRotator (Math|Conversions|ToQuaternion(Rotator) _impactnormal)))
  (return _returnvalue_2))