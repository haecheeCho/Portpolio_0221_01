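; Dual-wield attachment Blueprint that shows a pair of skeletal meshes in its owning character's hands while equipped.
; On equip, it attaches both meshes to the right and left dual hand sockets, disables their collision and makes them visible.
; BeginPlay and unequip share logic that hides both meshes without detaching them; a one-hand holster attach node exists but never runs.
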(event EventOnEquip
  (bind _skeletalmesh (Variables|Default|GetSkeletalMesh))
  (bind _skeletalmesh1 (Variables|Default|GetSkeletalMesh1))
  (|CallParentFunction)
  (bind _ascharacter (Utilities|Casting|CastToCharacter (Components|GetOwner)))
  (Transformation|AttachComponentToComponent _skeletalmesh (Variables|/Script/Engine.Character|GetMesh _ascharacter) "Hand_Dual_R" "KeepRelative" "KeepRelative" "KeepRelative" true)
  (Transformation|AttachComponentToComponent _skeletalmesh1 (Variables|/Script/Engine.Character|GetMesh _ascharacter) "Hand_Dual_L" "KeepRelative" "KeepRelative" "KeepRelative" true)
  (Collision|SetCollisionEnabled _skeletalmesh "NoCollision")
  (Collision|SetCollisionEnabled _skeletalmesh1 "NoCollision")
  (Rendering|SetVisibility (Variables|Default|GetSkeletalMesh) true true)
  (Rendering|SetVisibility (Variables|Default|GetSkeletalMesh1) true true))

(event EventOnUnequip
  (|CallParentFunction)
  (bind _ascharacter (Utilities|Casting|CastToCharacter (Components|GetOwner)))
  (Rendering|SetVisibility (Variables|Default|GetSkeletalMesh) false false)
  (Rendering|SetVisibility (Variables|Default|GetSkeletalMesh1) false false))

(event EventBeginPlay
  (|CallParentFunction)
  (bind _ascharacter (Utilities|Casting|CastToCharacter (Components|GetOwner)))
  (Rendering|SetVisibility (Variables|Default|GetSkeletalMesh) false false)
  (Rendering|SetVisibility (Variables|Default|GetSkeletalMesh1) false false))

(fn ConstructionScript
  (|CallParentFunction))