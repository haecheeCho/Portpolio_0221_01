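; Throw action Blueprint that makes the owning character launch a projectile as part of an action system.
; DoAction runs only from idle, switching the state to action mode and playing the first action entry.
; BeginDoAction spawns that entry's throw class at the Hand_IceBall socket, facing the character's forward vector, and passes it the action data.
; EndDoAction returns the state to idle.
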(fn ConstructionScript
  (|CallParentFunction))

(fn DoAction
  (bind _state (Variables|Default|GetState))
  (|CallParentFunction)
  (if (Default|IsIdleMode _state)
    (Default|SetActionMode _state)
    (CallFunction|PlayAction)))

(fn BeginDoAction
  (bind _datas (Variables|Default|GetDatas))
  (bind _output (Utilities|Array|Get(acopy) _datas))
  (|CallParentFunction)
  (bind _returnvalue (Game|SpawnActorfromClass (.ThrowClass (Utilities|Struct|BreakFDoAcionData _output)) (Math|Transform|MakeTransform (Transformation|GetSocketLocation (Variables|/Script/Engine.Character|GetMesh (Variables|Default|GetOwnerCharacter)) "Hand_IceBall") (Class|KismetMathLibrary|QuatRotator (Math|Conversions|ToQuaternion(Rotator) (Transformation|GetActorForwardVector (Variables|Default|GetOwnerCharacter))))) "AlwaysSpawn" (Variables|Default|GetOwnerCharacter) 0))
  (Utilities|IsValid _returnvalue
    (:Is%20Valid
      (Variables|/Game/Actions/BP_Throw.BP_Throw_C|SetData _returnvalue _output))))

(fn EndDoAction
  (|CallParentFunction)
  (Default|SetIdleMode (Variables|Default|GetState)))

(fn PlaySound
  (|CallParentFunction))