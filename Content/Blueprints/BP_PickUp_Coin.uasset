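; BP_PickUp_Coin is a collectible coin actor that adds to the coin count when something overlaps its Sphere.
; The overlap prints a debug string and increments Coin on GM_ThirdPersonGamemode before checking what overlapped.
; Only if the other actor is BP_Player does it refresh that player's status widget, play the coin sound and destroy itself.
; Non-player overlaps therefore still raise the count and leave the coin in place.
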(event OnComponentBeginOverlap(Sphere)
  (params (OverlappedComponent :type Primitive%20Component%20Object%20Reference) (OtherActor :type Actor%20Object%20Reference) (OtherComp :type Primitive%20Component%20Object%20Reference) (OtherBodyIndex :type Integer) (bFromSweep :type Boolean) (SweepResult :type Hit%20Result%20Structure%20%28by%20ref%29))
  (Development|PrintString "Hello")
  (bind _asgm_third_person_gamemode (Utilities|Casting|CastToGM_ThirdPersonGamemode (Game|GetGameMode)))
  (bind _result (Math|Integer|IncrementInt (Variables|/Game/Player/GM_ThirdPersonGamemode.GM_ThirdPersonGamemode_C|GetCoin _asgm_third_person_gamemode))
    (:%20%20
      (Variables|/Game/Player/GM_ThirdPersonGamemode.GM_ThirdPersonGamemode_C|SetCoin _asgm_third_person_gamemode _result)
      (bind _asbp_player (Utilities|Casting|CastToBP_Player OtherActor))
      (Default|UpdateCoin (Variables|/Game/Player/BP_Player.BP_Player_C|GetStatusWidget _asbp_player))
      (Audio|PlaySoundatLocation "/Game/Sound/Coin.Coin" (Transformation|GetActorLocation self) "0, 0, 0" 0.5 1.0 0.0 0 0 0)
      (Actor|DestroyActor))))

(event EventBeginPlay
  (|CallParentFunction) ; 지금 이 노드는 비활성 상태입니다. \n핀을 끌어서 다른 노드를 연결하면 활성화됩니다.
)

(event Collision|EventActorBeginOverlap
  (params (OtherActor :type Actor%20Object%20Reference))
  (|CallParentFunction OtherActor) ; 지금 이 노드는 비활성 상태입니다. \n핀을 끌어서 다른 노드를 연결하면 활성화됩니다.
)

(event EventTick
  (params (DeltaSeconds :type Float%20%28single-precision%29))
  (|CallParentFunction DeltaSeconds) ; 지금 이 노드는 비활성 상태입니다. \n핀을 끌어서 다른 노드를 연결하면 활성화됩니다.
)

(fn ConstructionScript
  (|CallParentFunction))