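; Attachment Blueprint for a two-handed item that moves between holster and hand on the owning Character's mesh.
; It attaches to the Holster_TwoHand socket on BeginPlay and on unequip, and to Hand_TwoHand on equip.
; Each event calls its parent first, then attaches with relative transforms kept, provided the owner is a Character.
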(event EventOnEquip
  (|CallParentFunction)
  (bind _ascharacter (Utilities|Casting|CastToCharacter (Components|GetOwner)))
  (Transformation|AttachComponentToComponent (Variables|/Script/Engine.Character|GetMesh _ascharacter) "Hand_TwoHand" "KeepRelative" "KeepRelative" "KeepRelative" true))

(event EventOnUnequip
  (|CallParentFunction)
  (bind _ascharacter (Utilities|Casting|CastToCharacter (Components|GetOwner)))
  (Transformation|AttachComponentToComponent (Variables|/Script/Engine.Character|GetMesh _ascharacter) "Holster_TwoHand" "KeepRelative" "KeepRelative" "KeepRelative" true))

(event EventBeginPlay
  (|CallParentFunction)
  (bind _ascharacter (Utilities|Casting|CastToCharacter (Components|GetOwner)))
  (Transformation|AttachComponentToComponent (Variables|/Script/Engine.Character|GetMesh _ascharacter) "Holster_TwoHand" "KeepRelative" "KeepRelative" "KeepRelative" true))

(fn ConstructionScript
  (|CallParentFunction))