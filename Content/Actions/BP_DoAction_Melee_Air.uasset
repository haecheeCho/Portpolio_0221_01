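; Melee action, named as the air variant, that plays an indexed combo chain for the owning character.
; DoAction starts the first attack from idle or queues the next within the combo window, and BeginDoAction advances to it.
; Attachment overlaps damage each character once per swing via a hit list, using the current index, which also selects sounds.
; Ending resets index, state, movement and hit list, then blends the camera back to the owner.
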(fn ConstructionScript
  (|CallParentFunction))

(fn DoAction
  (bind _state (Variables|Default|GetState))
  (|CallParentFunction)
  (if (Variables|Default|GetEnable)
    (Variables|Default|SetExist true)
    (Variables|Default|SetEnable false)
    (elif (Default|IsIdleMode _state)
      (Default|SetActionMode _state)
      (CallFunction|PlayAction))))

(fn BeginDoAction
  (|CallParentFunction)
  (if (Variables|Default|GetExist)
    (Variables|Default|SetExist false)
    (Animation|StopAnimMontage (Variables|Default|GetOwnerCharacter) 0)
    (bind _result (Math|Integer|IncrementInt (Variables|Default|GetIndex))
      (:%20%20
        (CallFunction|PlayAction _result)
        (Utilities|Array|Clear (Variables|Default|GetHittedCharacters))))))

(fn EndDoAction
  (|CallParentFunction)
  (Animation|StopAnimMontage (Variables|Default|GetOwnerCharacter) 0)
  (Variables|Default|SetIndex 0)
  (Default|SetIdleMode (Variables|Default|GetState))
  (Default|SetMove (Variables|Default|GetStatus))
  (Utilities|Array|Clear (Variables|Default|GetHittedCharacters))
  (Game|Player|SetViewTargetwithBlend (Game|GetPlayerController 0) (Variables|Default|GetOwnerCharacter) 0.6 "VTBlend_Linear" 0.0 false))

(fn OnCombo
  (Variables|Default|SetEnable true))

(fn OffCombo
  (Variables|Default|SetEnable false))

(fn OnAttachmentBeginOverlap
  (params (OtherCharacter :type Character%20Object%20Reference))
  (|CallParentFunction OtherCharacter)
  (if (< (Utilities|Array|FindItem (Variables|Default|GetHittedCharacters) OtherCharacter) 0)
    (Utilities|Array|Add (Variables|Default|GetHittedCharacters) OtherCharacter)
    (CallFunction|SendDamage OtherCharacter (Variables|Default|GetIndex))))

(fn HitStopTimer
  (Utilities|Time|SetGlobalTimeDilation 1.0))

(fn OnAttachmentEndOverlap
  (params (OtherCharacter :type Character%20Object%20Reference))
  (|CallParentFunction 0))

(fn ClearHitted
  (Utilities|Array|Clear (Variables|Default|GetHittedCharacters)))

(fn PlaySound
  (bind _index (Variables|Default|GetIndex))
  (|CallParentFunction)
  (if (<= _index (- (Utilities|Array|Length (Variables|Default|GetDatas)) 1))
    (Audio|PlaySoundatLocation (.sound (Utilities|Array|Get(acopy) (Variables|Default|GetDatas) _index)) (Transformation|GetActorLocation (Variables|Default|GetOwnerCharacter)) "0, 0, 0" 1.0 1.0 0.0 0 0 0)))