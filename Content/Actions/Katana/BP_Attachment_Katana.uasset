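; Katana weapon attachment that moves the blade and its scabbard (Saya) between sockets on the owning Character's mesh.
; On BeginPlay and OnUnequip, both components attach to the Saya socket.
; OnEquip puts the blade in the right hand and the scabbard in the left, while OffEquip returns only the scabbard to its socket.
; Each event calls its parent first, and all attachments keep relative transforms.
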(event EventOffEquip
  (|CallParentFunction)
  (bind _ascharacter (Utilities|Casting|CastToCharacter (Components|GetOwner)))
  (Transformation|AttachComponentToComponent (Variables|Default|GetSaya) (Variables|/Script/Engine.Character|GetMesh _ascharacter) "Saya" "KeepRelative" "KeepRelative" "KeepRelative" true))

(event EventOnEquip
  (|CallParentFunction)
  (bind _ascharacter (Utilities|Casting|CastToCharacter (Components|GetOwner)))
  (Transformation|AttachComponentToComponent (Variables|Default|GetKatana) (Variables|/Script/Engine.Character|GetMesh _ascharacter) "R_Hand_Weapon" "KeepRelative" "KeepRelative" "KeepRelative" true)
  (Transformation|AttachComponentToComponent (Variables|Default|GetSaya) (Variables|/Script/Engine.Character|GetMesh _ascharacter) "L_Hand_Weapon" "KeepRelative" "KeepRelative" "KeepRelative" true))

(event EventOnUnequip
  (|CallParentFunction)
  (bind _ascharacter (Utilities|Casting|CastToCharacter (Components|GetOwner)))
  (Transformation|AttachComponentToComponent (Variables|Default|GetKatana) (Variables|/Script/Engine.Character|GetMesh _ascharacter) "Saya" "KeepRelative" "KeepRelative" "KeepRelative" true)
  (Transformation|AttachComponentToComponent (Variables|Default|GetSaya) (Variables|/Script/Engine.Character|GetMesh _ascharacter) "Saya" "KeepRelative" "KeepRelative" "KeepRelative" true))

(event EventBeginPlay
  (|CallParentFunction)
  (bind _ascharacter (Utilities|Casting|CastToCharacter (Components|GetOwner)))
  (Transformation|AttachComponentToComponent (Variables|Default|GetKatana) (Variables|/Script/Engine.Character|GetMesh _ascharacter) "Saya" "KeepRelative" "KeepRelative" "KeepRelative" true)
  (Transformation|AttachComponentToComponent (Variables|Default|GetSaya) (Variables|/Script/Engine.Character|GetMesh _ascharacter) "Saya" "KeepRelative" "KeepRelative" "KeepRelative" true))

(fn ConstructionScript
  (|CallParentFunction))