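; Base action class for a character's attacks, with empty DoAction, begin/end, attachment-overlap and sound functions, likely for child overrides.
; BeginPlay caches the owning Character and its State and Status components.
; PlayAction reads an indexed Datas entry to launch the owner vertically, play a montage and set movement.
; SendDamage uses the same data for damage, effect, camera shake, vertical target launch and hit stop via global time dilation.
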(event EventBeginPlay
  (bind _ascharacter (Utilities|Casting|CastToCharacter (Components|GetOwner)))
  (bind _output_get (Variables|Default|SetOwnerCharacter _ascharacter))
  (Variables|Default|SetState (Actor|GetComponentbyClass _output_get "/Game/Components/StateComponent.StateComponent_C"))
  (Variables|Default|SetStatus (Actor|GetComponentbyClass _output_get "/Game/Components/StatusComponent.StatusComponent_C")))

(fn ConstructionScript)

(fn DoAction)

(fn BeginDoAction)

(fn EndDoAction)

(fn PlayAction
  (params (Index :type Integer))
  (bind _datas (Variables|Default|GetDatas))
  (bind _status (Variables|Default|GetStatus))
  (bind _output (Utilities|Array|Get(acopy) _datas Index))
  (if (<= Index (- (Utilities|Array|Length (Variables|Default|GetDatas)) 1))
    (CallFunction|Launch (.launch _output)) ; 이따 수정
    (Animation|PlayAnimMontage (Variables|Default|GetOwnerCharacter) (.animmontage _output) (.playratio _output) (.startsection _output))
    (if (.canmove _output)
      (Default|SetMove _status)
      (else
        (Default|SetStop _status)))))

(fn OnAttachmentBeginOverlap
  (params (OtherCharacter :type Character%20Object%20Reference)))

(fn OnAttachmentEndOverlap
  (params (OtherCharacter :type Character%20Object%20Reference)))

(fn GetEquipped
  (bind _ownercharacter (Variables|Default|GetOwnerCharacter))
  (bind _returnvalue (Actor|GetComponentbyClass _ownercharacter "/Game/Components/ActionComponent.ActionComponent_C"))
  (Utilities|IsValid _returnvalue
    (:Is%20Valid
      (return (Default|GetEquipped (Default|GetEquipment _returnvalue))))))

(fn SendDamage
  (params (OtherCharacter :type Character%20Object%20Reference) (Index :type Integer))
  (bind _datas (Variables|Default|GetDatas))
  (bind _datas_2 (Variables|Default|GetDatas))
  (bind _datas_3 (Variables|Default|GetDatas))
  (bind _output (Utilities|Array|Get(acopy) _datas Index))
  (bind _output_2 (Utilities|Array|Get(acopy) _datas_2 Index))
  (bind _output_3 (Utilities|Array|Get(acopy) _datas_3 Index))
  (bind (_location _rotation _scale) (Math|Transform|BreakTransform (.effecttransform _output_3)))
  (if (Utilities|Array|IsValidIndex (Variables|Default|GetDatas) Index)
    (Utilities|FlowControl|Sequence
      (:then_0
        (Game|Damage|ApplyDamage OtherCharacter (.power (Utilities|Array|Get(acopy) (Variables|Default|GetDatas) Index)) (Pawn|GetController (Variables|Default|GetOwnerCharacter)) self))
      (:then_1
        (Utilities|IsValid (.effect _output_3)
          (:Is%20Valid
            (Effects|SpawnEmitteratLocation (.effect _output_3) (+ (Transformation|GetActorLocation OtherCharacter) _location) "0, 0, 0" _scale))))
      (:then_2
        (if (Utilities|IsValidClass (.shakeclass _output))
          (Class|PlayerCameraManager|StartMatineeCameraShake (Variables|/Script/Engine.PlayerController|GetPlayerCameraManager (Game|GetPlayerController 0)) (.shakeclass _output) 1.0 "CameraLocal" "0, 0, 0")))
      (:then_3
        (if (> (.hitstop _output_2) 0.0)
          (Utilities|Time|SetGlobalTimeDilation 0.001)
          (Utilities|Time|SetTimerbyFunctionName self "HitStopTimer" (* (.hitstop _output_2) 0.001))))
      (:then_4
        (Character|LaunchCharacter OtherCharacter (Math|Vector|MakeVector 0.0 0.0 (.z (Math|Vector|RotateVector (.force (Utilities|Array|Get(acopy) (Variables|Default|GetDatas) Index)) (Math|Rotator|FindLookatRotation (Transformation|GetActorLocation (Variables|Default|GetOwnerCharacter)) (Transformation|GetActorLocation OtherCharacter))))) false true)))))

(fn Launch
  (params (z :type Float%20%28single-precision%29))
  (if true
    (Character|LaunchCharacter (Variables|Default|GetOwnerCharacter) (Math|Vector|MakeVector 0.0 0.0 z) false false)))

(fn PlaySound)