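; Flame throw magic action Blueprint that plays a cast montage and tracks characters to damage, apparently unfinished.
; DoAction switches an idle owner to action mode and plays the first action.
; Attachment overlaps maintain a hit list that OnHitted damages, but nothing here calls or schedules it.
; BeginDoAction only validates the attachment's sphere, and OnFinish's cleanup of visibility, timer, collision and idle state is disconnected.
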(event EventTick
  (params (DeltaSeconds :type Float%20%28single-precision%29)))

(fn ConstructionScript
  (|CallParentFunction))

(fn DoAction
  (bind _state (Variables|Default|GetState))
  (if (Default|IsIdleMode _state)
    (Default|SetActionMode _state)
    (CallFunction|PlayAction)))

(fn BeginDoAction
  (if (Math|Boolean|ANDBoolean true true (Utilities|IsValid (CallFunction|GetSphere)))
    _))

(fn EndDoAction
  (|CallParentFunction))

(fn OnFinish)

(fn OnAttachmentBeginOverlap
  (params (OtherCharacter :type Character%20Object%20Reference))
  (Utilities|Array|AddUnique (Variables|Default|GetHittedCharacters) OtherCharacter))

(fn OnAttachmentEndOverlap
  (params (OtherCharacter :type Character%20Object%20Reference))
  (Utilities|Array|RemoveItem (Variables|Default|GetHittedCharacters) OtherCharacter))

(fn OnHitted
  (for _array_element (Variables|Default|GetHittedCharacters)
    (CallFunction|SendDamage _array_element)))

(fn GetSphere
  (bind _ownercharacter (Variables|Default|GetOwnerCharacter))
  (bind _returnvalue (Actor|GetComponentbyClass _ownercharacter "/Game/Components/ActionComponent.ActionComponent_C"))
  (bind _attachment (Default|GetAttachment _returnvalue))
  (bind _returnvalue_2 (Actor|GetComponentbyClass _attachment "/Script/Engine.SphereComponent"))
  (Utilities|IsValid _returnvalue
    (:Is%20Valid
      (Utilities|IsValid _returnvalue_2
        (:Is%20Valid
          (return _returnvalue_2))))))